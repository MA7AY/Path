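; In-game player controller that owns the MainUI widget and switches its screens along with cursor and input mode for game start, death and game end.
; BeginPlay opens the UI in UI-only input and caches the BP_Devvy pawn; startplay hands control to gameplay.
; Tick pushes stamina and health to the widget and polls HP to toggle between gameplay and Game Over.
; SpawnPers spawns and possesses a new BP_Devvy at the first PlayerStart found.
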(event `self.ReceiveBeginPlay`
  (`|ExecutionSequence`
    (:`then_0`
      (bind _returnvalue (`|CreateWidget` "/Game/Main/UI/MainUI.MainUI_C"))
      (set `self.MainWidget` _returnvalue)
      (`UserWidget.AddToViewport` (`self.MainWidget`) 0)
      (set `self.bShowMouseCursor` true)
      (`WidgetBlueprintLibrary.SetInputMode_UIOnlyEx` self (`self.MainWidget`)))
    (:`then_1`
      (bind _asbp_devvy (cast `/Game/Main/Blueprints/BP_Devvy` (`self.K2_GetPawn`)))
      (set `self.MyPawn` _asbp_devvy))))

(event `startplay`
  (`/Game/Main/UI/MainUI.SwitchScreen` (`self.MainWidget`) 1)
  (set `self.bShowMouseCursor` false)
  (`WidgetBlueprintLibrary.SetInputMode_GameOnly` self))

(event `self.ReceiveTick`
  (params (DeltaSeconds :type "Float (single-precision)"))
  (bind _mypawn (`self.MyPawn`))
  (bind _statusac (`/Game/Main/Blueprints/BP_Devvy.StatusAC` (`self.MyPawn`)))
  (`|ExecutionSequence`
    (:`then_0`
      (`/Game/Main/UI/MainUI.UpdateStamina` (`self.MainWidget`) (`/Game/Main/Blueprints/BP_Devvy.MaxStamina` _mypawn) (`/Game/Main/Blueprints/BP_Devvy.Stamina` _mypawn)))
    (:`then_1`
      (`/Game/Main/UI/MainUI.UpdateHealth` (`self.MainWidget`) (`/Game/Main/Blueprints/StatusAC.CurrentHP` _statusac) (`/Game/Main/Blueprints/StatusAC.MaxHP` _statusac)))
    (:`then_2`
      ;[1 1 1] Проверка жив игрок или нет
      (if (`self.playerAlive`)
        ;[1 1 1] Если жив и здоровье меньше 0 то делаем мертвым
        (if (<= (`/Game/Main/Blueprints/StatusAC.CurrentHP` (`/Game/Main/Blueprints/BP_Devvy.StatusAC` (`self.MyPawn`))) 0.0)
          (set `self.playerAlive` false)
          ;[1 1 1] Изменяем игровое окно на GameOver
          (`/Game/Main/UI/MainUI.SwitchScreen` (`self.MainWidget`) 2)
          ;[1 1 1] Включаем видимость курсора
          (set `self.bShowMouseCursor` true)
          ;[1 1 1] Изменяем режим ввода данных на "только с виджетов"
          (`WidgetBlueprintLibrary.SetInputMode_UIOnlyEx` self (`self.MainWidget`)))
        (else
          ;[1 1 1] Если павн мертв и его здоровье больше 0 то делаем его живым
          (if (> (`/Game/Main/Blueprints/StatusAC.CurrentHP` (`/Game/Main/Blueprints/BP_Devvy.StatusAC` (`self.MyPawn`))) 0.0)
            (set `self.PlayerAlive` true)
            ;[1 1 1] Преключаем окно на GamrPlay
            (`/Game/Main/UI/MainUI.SwitchScreen` (`self.MainWidget`) 1)
            ;[1 1 1] Убираем курсор
            (set `self.bShowMouseCursor` false)
            ;[1 1 1] Изменяем режим вводв данных на только с клавишь
            (`WidgetBlueprintLibrary.SetInputMode_GameOnly` self)))))))

(event `SpawnPers`
  ;[1 1 1] Спаун
  (bind _outactors (`GameplayStatics.GetAllActorsOfClass` "/Script/Engine.PlayerStart"))
  (bind _returnvalue (`|SpawnActorFromClass` "/Game/Main/Blueprints/BP_Devvy.BP_Devvy_C" (`self.GetTransform` (`|GetArrayItem` _outactors)) "AlwaysSpawn" "OverrideRootScale" null null))
  (set `self.MyPawn` _returnvalue)
  (`self.UnPossess`)
  (`self.Possess` (`self.MyPawn`)))

(event `EndGame`
  (`/Game/Main/UI/MainUI.SwitchScreen` (`self.MainWidget`) 3)
  (set `self.bShowMouseCursor` true)
  (`WidgetBlueprintLibrary.SetInputMode_UIOnlyEx` self (`self.MainWidget`)))

(fn `UserConstructionScript`)