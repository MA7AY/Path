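; StatusAC is a status component that tracks health and handles damage, judging by its name and functions.
; It fills CurrentHP from MaxHP on BeginPlay, and MakeDamageHealth subtracts damage clamped between zero and MaxHP.
; The OnDead dispatcher fires whenever a damage call leaves health at zero, with no guard against repeat calls.
; Tick prints the current health on screen every frame as debug output.
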(event `self.ReceiveBeginPlay`
  (set `self.CurrentHP` (`self.MaxHP`)))

(event `self.ReceiveTick`
  (params (DeltaSeconds :type "Float (single-precision)"))
  (`KismetSystemLibrary.PrintString` (`KismetStringLibrary.Conv_DoubleToString` (`self.CurrentHP`)) true true (struct :`G` 0.66 :`B` 1.0 :`A` 1.0) DeltaSeconds))

(fn `MakeDamage/Health`
  (params (Value :type "Float (double-precision)"))
  ;[1 1 1] Функция наносит урон
  (set `self.CurrentHP` (`KismetMathLibrary.FClamp` (- (`self.CurrentHP`) Value) 0.0 (`self.MaxHP`)))
  (if (<= (`self.CurrentHP`) 0.0)
    (`self.OnDead`)))